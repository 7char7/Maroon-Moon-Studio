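; BP_Stalker is an AI pawn that wanders the level and investigates noises.
; A looping timer set on BeginPlay calls Roam, which uses AI MoveTo toward a random navigable point within a radius of its current location.
; PawnSensing's hearing event sends it to the noise instigator's location, while the roam timer keeps running and can redirect it.
; Both behaviors print debug text.
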(event `self.PawnSensing.OnHearNoise`
  (params (Instigator :type "Pawn Object Reference") (Location :type "Vector Structure (by ref)") (Volume :type "Float (single-precision)"))
  ; Goes to a sound it hears, any sound so car alarm, thrown object, play steps
  (`KismetSystemLibrary.PrintText` "Hello")
  (`|AIMoveTo` self (`self.K2_GetActorLocation` Instigator) null))

(event `Roam`
  ; Ai will roam around, picks random spot in radius and goes to it, called from event play
  (`KismetSystemLibrary.PrintText` "roam")
  (bind _randomlocation (`NavigationSystemV1.K2_GetRandomLocationInNavigableRadius` (`self.K2_GetActorLocation`) 1000.0 null null))
  (`|AIMoveTo` self _randomlocation null))

(event `self.ReceiveBeginPlay`
  ; Calls roam function on a timer, 5 secs right nw
  (`KismetSystemLibrary.K2_SetTimer` null "Roam" 5.0 true))

(fn `UserConstructionScript`)