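; Component that runs a button-mash quick-time event, likely to break out of a Stalker's hold, and reports success or failure through CallCompleted.
; BeginPlay shows a WB_Spam_Bar prompt for Q with a randomized press target, and each press advances the bar.
; It fails if nothing is pressed within five seconds or a retriggerable delay, restarted by any key release, expires.
; Either outcome removes the widget and destroys the component.
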(event `self.ReceiveBeginPlay`
  ; Core mechanic setup/The spam button will be "Q"
  (bind _returnvalue (`|CreateWidget` "/Game/Blueprints/Stalker/WB_Spam_Bar.WB_Spam_Bar_C"))
  (set `self.WidgetRefernce` _returnvalue)
  (`UserWidget.AddToViewport` (`self.WidgetRefernce`) 0)
  (set `self.NeededAmount` (`KismetMathLibrary.RandomFloatInRange` 10.0 15.0))
  (set `self.KeyPressed` (select `int` (`KismetMathLibrary.RandomInteger` 2) :`0` "Q" :`1` "Q" :`2` "Gamepad_FaceButton_Left" :!type "Key Structure"))
  (`TextBlock.SetText` (`/Game/Blueprints/Stalker/WB_Spam_Bar.SpamText` (`self.WidgetRefernce`)) (`|FormatText` "Spam {Key}" (`KismetInputLibrary.Key_GetDisplayName` (`self.KeyPressed`))))
  (`self.UpdateProgressBar`)
  ; If bar is not filled in 5 seconds, it fails
  (`KismetSystemLibrary.Delay` 5.0)
  (`/Engine/EditorBlueprintResources/StandardMacros.IsValid` self
    (:`Is Valid`
      (if (<= (`self.AmountPressed`) 0.0)
        (`self.OnFailed`)))))

(event `PressKey`
  (set `self.AmountPressed` (`KismetMathLibrary.FClamp` (+ (`self.AmountPressed`) 1.0) 0.0 (`self.NeededAmount`)))
  (`self.UpdateProgressBar`)
  (if (== (`self.AmountPressed`) (`self.NeededAmount`))
    (`self.Completed` true)
    (`self.Destroy`)))

(event `ReleaseKey`
  ; How many seconds the player can not spam the button before failing
  (`KismetSystemLibrary.RetriggerableDelay` 0.7)
  (`self.OnFailed`))

(event `OnFailed`
  (set `self.AmountPressed` 0.0)
  (`self.UpdateProgressBar`)
  (`self.Completed` false)
  (`self.Destroy`))

(event `Destroy`
  (bind _widgetrefernce (`self.WidgetRefernce`)
    (:`then`
      (`Widget.RemoveFromParent` _widgetrefernce))
    (:`else`
      _))
  (`self.K2_DestroyComponent`))

(event `Key|AnyKey`
  (params (Key :type "Key Structure"))
  (:`Pressed`
    (if (== Key (`self.KeyPressed`))
      (`self.PressKey`)))
  (:`Released`
    (`self.ReleaseKey`)))

(fn `UpdateProgressBar`
  (`ProgressBar.SetPercent` (`/Game/Blueprints/Stalker/WB_Spam_Bar.SpamBar` (`self.WidgetRefernce`)) (/ (`self.AmountPressed`) (`self.NeededAmount`))))