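; BP_NPC2 is an NPC that the player can talk to, stepping through a list of dialogue lines.
; Each Talk event advances TalkIndex and writes that Dialogue entry into a WB_Dialogue2 widget, created when none is valid and removed once the lines run out.
; A TriggerZone shows the interaction prompt widget on overlap and hides it when the overlap ends.
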(event `self.Talk`
  ; Dialogue mechanic
  (`/Engine/EditorBlueprintResources/StandardMacros.IncrementInt` (`self.TalkIndex`)
    (:`  `
      (if (< (`self.TalkIndex`) (`KismetArrayLibrary.Array_Length` (`self.dialogue`)))
        (`self.UI`
          (:`then`
            _)
          (:`else`
            (`|CreateWidget` "/Game/Blueprints/NPCs/WB_Dialogue2.WB_Dialogue2_C" (`GameplayStatics.GetPlayerController` 0))
            (bind _output_get (set `self.UI` null))
            (`UserWidget.AddToViewport` _output_get 0)))
        (`TextBlock.SetText` (`/Game/Blueprints/NPCs/WB_Dialogue.TalkText` (`self.UI`)) (`KismetTextLibrary.Conv_StringToText` (`|GetArrayItem` (`self.dialogue`) (`self.TalkIndex`))))
        (else
          (`Widget.RemoveFromParent` (`self.UI`)))))))

(event `self.Trigger Zone.OnComponentBeginOverlap`
  (params (OverlappedComponent :type "PrimitiveComponent Object Reference") (OtherActor :type "Actor Object Reference") (OtherComp :type "PrimitiveComponent Object Reference") (OtherBodyIndex :type Integer) (bFromSweep :type Boolean) (SweepResult :type "HitResult Structure (by ref)"))
  ; Dialogue interaction ui trigger
  (`SceneComponent.SetVisibility` (`self.Widget`) true false))

(event `self.Trigger Zone.OnComponentEndOverlap`
  (params (OverlappedComponent :type "PrimitiveComponent Object Reference") (OtherActor :type "Actor Object Reference") (OtherComp :type "PrimitiveComponent Object Reference") (OtherBodyIndex :type Integer))
  ; Dialogue interaction ui trigger
  (`SceneComponent.SetVisibility` (`self.Widget`) false false))

(fn `UserConstructionScript`)