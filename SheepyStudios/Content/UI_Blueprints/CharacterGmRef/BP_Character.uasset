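; BP_Character is the player character, handling movement, look, menus and evidence interaction.
; BeginPlay pre-creates collapsed phone menu, evidence, NPC and text log widgets, creating the NPC log twice and keeping only the second reference.
; Pause creates a fresh menu and PhoneMenu reveals the existing one; both pause the game with cursor and UI-only input.
; Interact sends StartPhotoInteractionMessage to overlapping CollectEvidenceExample actors implementing BPI_PhotoInteract.
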(event `InputAxis|Forward`
  (params (AxisValue :type "Float (single-precision)"))
  (`self.AddMovementInput` (`SceneComponent.GetForwardVector` (`self.CapsuleComponent`)) AxisValue))

(event `InputAxis|Right`
  (params (AxisValue :type "Float (single-precision)"))
  (`self.AddMovementInput` (`SceneComponent.GetRightVector` (`self.CapsuleComponent`)) AxisValue))

(event `InputAxis|Pitch`
  (params (AxisValue :type "Float (single-precision)"))
  ; Camera View
  (`self.AddControllerPitchInput` AxisValue))

(event `InputAxis|Yaw`
  (params (AxisValue :type "Float (single-precision)"))
  ; Camera View
  (`self.AddControllerYawInput` AxisValue))

(event `InputAction|Pause`
  (params (Key :type "Key Structure"))
  (bind _returnvalue (`GameplayStatics.GetPlayerController` 0))
  ; Pause Menu
  (:`Pressed`
    (bind _returnvalue_2 (`|CreateWidget` "/Game/UI_Blueprints/PauseMenu/WBP_PauseMenu.WBP_PauseMenu_C"))
    (`UserWidget.AddToViewport` _returnvalue_2 0)
    (set `PlayerController.bShowMouseCursor` true _returnvalue)
    (`WidgetBlueprintLibrary.SetInputMode_UIOnlyEx` _returnvalue null)
    (`GameplayStatics.SetGamePaused` true)))

(event `InputAction|PhoneMenu`
  (params (Key :type "Key Structure"))
  (bind _returnvalue (`GameplayStatics.GetPlayerController` 0))
  ; Phone Menu
  (:`Pressed`
    (`Widget.SetVisibility` (`self.Phone Menu Widget `) "Visible")
    (set `PlayerController.bShowMouseCursor` true _returnvalue)
    (`WidgetBlueprintLibrary.SetInputMode_UIOnlyEx` _returnvalue null)
    (`GameplayStatics.SetGamePaused` true)))

(event `self.ReceiveBeginPlay`
  (bind _returnvalue (`|CreateWidget` "/Game/UI_Blueprints/PhoneMenu/WBP_PhoneMenu.WBP_PhoneMenu_C"))
  (bind _output_get (set `self.Phone Menu Widget ` _returnvalue))
  (`UserWidget.AddToViewport` _output_get 0)
  (`Widget.SetVisibility` (`self.Phone Menu Widget `) "Collapsed")
  (bind _returnvalue_2 (`|CreateWidget` "/Game/UI_Blueprints/PhoneMenu/WBP_EvidenceLog.WBP_EvidenceLog_C"))
  (bind _output_get_2 (set `self.EvidenceLog` _returnvalue_2))
  (`UserWidget.AddToViewport` _output_get_2 0)
  (`Widget.SetVisibility` (`self.EvidenceLog`) "Collapsed")
  (bind _returnvalue_3 (`|CreateWidget` "/Game/UI_Blueprints/PhoneMenu/WBP_NpcLog.WBP_NpcLog_C"))
  (bind _output_get_3 (set `self.NPCLog` _returnvalue_3))
  (`UserWidget.AddToViewport` _output_get_3 0)
  (`Widget.SetVisibility` (`self.NPCLog`) "Collapsed")
  (bind _returnvalue_4 (`|CreateWidget` "/Game/UI_Blueprints/PhoneMenu/WBP_NpcLog.WBP_NpcLog_C"))
  (bind _output_get_4 (set `self.NPCLog` _returnvalue_4))
  (`UserWidget.AddToViewport` _output_get_4 0)
  (`Widget.SetVisibility` (`self.NPCLog`) "Collapsed")
  (bind _returnvalue_5 (`|CreateWidget` "/Game/UI_Blueprints/PhoneMenu/WBP_TextLog.WBP_TextLog_C"))
  (bind _output_get_5 (set `self.TextLog` _returnvalue_5))
  (`UserWidget.AddToViewport` _output_get_5 0)
  (`Widget.SetVisibility` (`self.TextLog`) "Collapsed"))

(event `InputAction|Interact`
  (params (Key :type "Key Structure"))
  (:`Pressed`
    (for _array_element (`self.GetOverlappingActors` "/Game/UI_Blueprints/PhoneMenu/CollectEvidenceExample.CollectEvidenceExample_C")
      (if (`KismetSystemLibrary.DoesImplementInterface` _array_element "/Game/UI_Blueprints/TakePhoto/BPI_PhotoInteract.BPI_PhotoInteract_C")
        (message `/Game/UI_Blueprints/TakePhoto/BPI_PhotoInteract.StartPhotoInteraction` _array_element)))))

(fn `UserConstructionScript`)